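; Mission Blueprint for "Sugary Sweet", which runs its linear objective chain from speaking with Roland through fleeing the factory to completion.
; After a short delay on BeginPlay it registers a starter callback with the player's MissionSystemComponent, then sets the first objective if the mission is active.
; Each listener event advances the objective enum one step, converts it to an integer, and updates HUD text and waypoint.
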(event Custom|MissionStarterActivator_Event_0
  (bind _missionisactive (CallFunction|CheckifMissionIsActive "NewEnumerator4"))
  (if _missionisactive
    (Variables|Default|SetMissionObjectives "NewEnumerator1")
    (Utilities|EnumIntegerUpdate)
    (CallFunction|UpdateHUDTitleandObjective (Variables|Default|GetSugary%20Sweet) (Variables|Default|GetSpeak%20with%20Roland%20%2801%29))
    (Default|CallMissionWaypointUpdate)))

(event EventBeginPlay
  (Utilities|FlowControl|Delay 1.0)
  (bind _asfirst_person_character (Utilities|Casting|CastToFirstPersonCharacter (Game|Player|GetPlayerPawn 0)))
  (Variables|Default|SetPlayerRef _asfirst_person_character)
  (Variables|Default|SetMOHUDRef (Variables|/Game/_FirstPersonBaseFiles/ProjectBasics/FirstPersonCharacter.FirstPersonCharacter_C|GetMissionObjectives_HUD _asfirst_person_character))
  (EventDispatchers|AssignMissionStarterActivator (Variables|/Game/_FirstPersonBaseFiles/ProjectBasics/FirstPersonCharacter.FirstPersonCharacter_C|GetMissionSystem_Component (Variables|Default|GetPlayerRef)) (delegate Custom|MissionStarterActivator_Event_0))
  (bind _missionisactive (CallFunction|CheckifMissionIsActive "NewEnumerator4"))
  (if _missionisactive
    (Variables|Default|SetMissionObjectives "NewEnumerator1")
    (Utilities|EnumIntegerUpdate)
    (CallFunction|UpdateHUDTitleandObjective (Variables|Default|GetSugary%20Sweet) (Variables|Default|GetSpeak%20with%20Roland%20%2801%29))
    (Default|CallMissionWaypointUpdate)))

(event EventMissionObserverListenerEvent
  (switch Utilities|FlowControl|Switch|SwitchonBP_Enum_SugarySweet (Variables|Default|GetMissionObjectives)
    (:NewEnumerator1
      (Variables|Default|SetMissionObjectives "NewEnumerator2")
      (Utilities|EnumIntegerUpdate)
      (CallFunction|UpdateHUDTitleandObjective (Variables|Default|GetSugary%20Sweet) (Variables|Default|GetFollow%20the%20guide%20%2801%29))
      (Default|CallMissionWaypointUpdate))
    (:NewEnumerator2
      (Variables|Default|SetMissionObjectives "NewEnumerator3")
      (Utilities|EnumIntegerUpdate)
      (CallFunction|UpdateHUDTitleandObjective (Variables|Default|GetSugary%20Sweet) (Variables|Default|GetGet%20the%20Eridium))
      (Default|CallMissionWaypointUpdate))
    (:NewEnumerator3
      (Variables|Default|SetMissionObjectives "NewEnumerator4")
      (Utilities|EnumIntegerUpdate)
      (CallFunction|UpdateHUDTitleandObjective (Variables|Default|GetSugary%20Sweet) (Variables|Default|GetGet%20back%20to%20the%20hub))
      (Default|CallMissionWaypointUpdate))
    (:NewEnumerator4
      (Variables|Default|SetMissionObjectives "NewEnumerator5")
      (Utilities|EnumIntegerUpdate)
      (CallFunction|UpdateHUDTitleandObjective (Variables|Default|GetSugary%20Sweet) (Variables|Default|GetSpeak%20with%20Roland%20%2802%29))
      (Default|CallMissionWaypointUpdate))
    (:NewEnumerator5
      (Variables|Default|SetMissionObjectives "NewEnumerator6")
      (Utilities|EnumIntegerUpdate)
      (CallFunction|UpdateHUDTitleandObjective (Variables|Default|GetSugary%20Sweet) (Variables|Default|GetFollow%20the%20guide%20%2802%29))
      (Default|CallMissionWaypointUpdate))
    (:NewEnumerator6
      (Variables|Default|SetMissionObjectives "NewEnumerator7")
      (Utilities|EnumIntegerUpdate)
      (CallFunction|UpdateHUDTitleandObjective (Variables|Default|GetSugary%20Sweet) (Variables|Default|GetSurvive%20the%20storm))
      (Default|CallMissionWaypointUpdate))
    (:NewEnumerator7
      (Variables|Default|SetMissionObjectives "NewEnumerator8")
      (Utilities|EnumIntegerUpdate)
      (CallFunction|UpdateHUDTitleandObjective (Variables|Default|GetSugary%20Sweet) (Variables|Default|GetComplete%20the%20witch's%20tasks))
      (Default|CallMissionWaypointUpdate))
    (:NewEnumerator8
      (Variables|Default|SetMissionObjectives "NewEnumerator9")
      (Utilities|EnumIntegerUpdate)
      (CallFunction|UpdateHUDTitleandObjective (Variables|Default|GetSugary%20Sweet) (Variables|Default|Get"Repair"%20the%20oven))
      (Default|CallMissionWaypointUpdate))
    (:NewEnumerator9
      (Variables|Default|SetMissionObjectives "NewEnumerator10")
      (Utilities|EnumIntegerUpdate)
      (CallFunction|UpdateHUDTitleandObjective (Variables|Default|GetSugary%20Sweet) (Variables|Default|GetKill%20the%20witch))
      (Default|CallMissionWaypointUpdate))
    (:NewEnumerator10
      (Variables|Default|SetMissionObjectives "NewEnumerator11")
      (Utilities|EnumIntegerUpdate)
      (CallFunction|UpdateHUDTitleandObjective (Variables|Default|GetSugary%20Sweet) (Variables|Default|GetFind%20the%20keys))
      (Default|CallMissionWaypointUpdate))
    (:NewEnumerator11
      (Variables|Default|SetMissionObjectives "NewEnumerator12")
      (Utilities|EnumIntegerUpdate)
      (CallFunction|UpdateHUDTitleandObjective (Variables|Default|GetSugary%20Sweet) (Variables|Default|GetFree%20Tannis%20&%20Tiny%20Tina))
      (Default|CallMissionWaypointUpdate))
    (:NewEnumerator12
      (Variables|Default|SetMissionObjectives "NewEnumerator13")
      (Utilities|EnumIntegerUpdate)
      (CallFunction|UpdateHUDTitleandObjective (Variables|Default|GetSugary%20Sweet) (Variables|Default|GetFlee%20the%20factory))
      (Default|CallMissionWaypointUpdate))
    (:NewEnumerator13
      (Variables|Default|SetMissionObjectives "NewEnumerator15")
      (Utilities|EnumIntegerUpdate)
      (CallFunction|UpdateHUDTitleandObjective (Variables|Default|GetSugary%20Sweet) (Variables|Default|GetMissionEnd))
      (Default|CallMissionWaypointUpdate))))

(fn ConstructionScript
  (|CallParentFunction))