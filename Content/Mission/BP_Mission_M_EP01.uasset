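; Mission actor for EP01 that starts the mission's objective tracking once the player's mission system reports it active.
; After a short BeginPlay delay, it caches the player and objectives HUD and registers an activation callback with the player's MissionSystemComponent.
; Both BeginPlay and that callback check mission status, then set the objective enum and run EnumIntegerUpdate.
; That macro maps each objective state to an integer; no objective-specific gameplay is wired up.
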(event Custom|CheckIfMissionIsActivated
  (bind _missionisactive (CallFunction|CheckifMissionIsActive "NewEnumerator0"))
  (if _missionisactive
    (Variables|Default|SetEnum_MissionObjectives "NewEnumerator1")
    (Utilities|EnumIntegerUpdate)))

(event EventBeginPlay
  (Utilities|FlowControl|Delay 1.0)
  (bind _asfirst_person_character (Utilities|Casting|CastToFirstPersonCharacter (Game|Player|GetPlayerPawn 0)))
  (Variables|Default|SetPlayerRef _asfirst_person_character)
  (Variables|Default|SetMOHUDRef (Variables|/Game/_FirstPersonBaseFiles/ProjectBasics/FirstPersonCharacter.FirstPersonCharacter_C|GetMissionObjectives_HUD _asfirst_person_character))
  (EventDispatchers|AssignMissionStarterActivator (Variables|/Game/_FirstPersonBaseFiles/ProjectBasics/FirstPersonCharacter.FirstPersonCharacter_C|GetMissionSystem_Component (Variables|Default|GetPlayerRef)) (delegate Custom|CheckIfMissionIsActivated))
  (bind _missionisactive (CallFunction|CheckifMissionIsActive "NewEnumerator0"))
  (if _missionisactive
    (Variables|Default|SetEnum_MissionObjectives "NewEnumerator1")
    (Utilities|EnumIntegerUpdate)))

(event Collision|EventActorBeginOverlap
  (params (OtherActor :type Actor%20Object%20Reference))
  (|CallParentFunction OtherActor) ; This node is disabled and will not be called.\nDrag off pins to build functionality.
)

(event EventTick
  (params (DeltaSeconds :type Float%20%28single-precision%29))
  (|CallParentFunction DeltaSeconds) ; This node is disabled and will not be called.\nDrag off pins to build functionality.
)

(fn ConstructionScript
  (|CallParentFunction))