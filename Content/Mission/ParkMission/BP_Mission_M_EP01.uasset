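; Mission actor for the park mission "It's a small world" (EP01), tracking objective progress for the player.
; After a short BeginPlay delay it registers with the player's MissionSystemComponent and starts Objective 1 if the mission is active.
; An observer listener and a custom event advance it to Objectives 2 and 3.
; Each step mirrors the objective enum into an integer via a macro, then updates HUD text and the waypoint.
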(event Custom|CheckIfMissionIsActivated
  (bind _missionisactive (CallFunction|CheckifMissionIsActive "NewEnumerator0"))
  (if _missionisactive
    (Variables|Default|SetEnum_MissionObjectives "NewEnumerator1")
    (Utilities|EnumIntegerUpdate
      (:Output
        (CallFunction|UpdateHUDTitleandObjective "It's a small world" (Variables|Default|GetObjective%201))
        (Default|CallMissionWaypointUpdate)))))

(event Custom|CustomEvent
  (switch Utilities|FlowControl|Switch|SwitchonEnum_MainMission1_Objectives (Variables|Default|GetMissionObjectives)
    (:NewEnumerator2
      (Variables|Default|SetMissionObjectives "NewEnumerator3")
      (Utilities|EnumIntegerUpdate
        (:Output
          (CallFunction|UpdateHUDTitleandObjective "It's a small world" (Variables|Default|GetObjective%203))
          (Default|CallMissionWaypointUpdate))))))

(event EventBeginPlay
  (Utilities|FlowControl|Delay 1.0)
  (bind _asfirst_person_character (Utilities|Casting|CastToFirstPersonCharacter (Game|Player|GetPlayerPawn 0)))
  (Variables|Default|SetPlayerRef _asfirst_person_character)
  (Variables|Default|SetMOHUDRef (Variables|/Game/_FirstPersonBaseFiles/ProjectBasics/FirstPersonCharacter.FirstPersonCharacter_C|GetMissionObjectives_HUD _asfirst_person_character))
  (EventDispatchers|AssignMissionStarterActivator (Variables|/Game/_FirstPersonBaseFiles/ProjectBasics/FirstPersonCharacter.FirstPersonCharacter_C|GetMissionSystem_Component (Variables|Default|GetPlayerRef)) (delegate Custom|CheckIfMissionIsActivated))
  (bind _missionisactive (CallFunction|CheckifMissionIsActive "NewEnumerator0"))
  (if _missionisactive
    (Variables|Default|SetEnum_MissionObjectives "NewEnumerator1")
    (Utilities|EnumIntegerUpdate
      (:Output
        (CallFunction|UpdateHUDTitleandObjective "It's a small world" (Variables|Default|GetObjective%201))
        (Default|CallMissionWaypointUpdate)))))

(event EventMissionObserverListenerEvent
  (switch Utilities|FlowControl|Switch|SwitchonEnum_MainMission1_Objectives (Variables|Default|GetMissionObjectives)
    (:NewEnumerator1
      (Variables|Default|SetMissionObjectives "NewEnumerator2")
      (Utilities|EnumIntegerUpdate
        (:Output
          (CallFunction|UpdateHUDTitleandObjective "It's a small world" (Variables|Default|GetObjective%202))
          (Default|CallMissionWaypointUpdate))))))

(fn ConstructionScript
  (|CallParentFunction))