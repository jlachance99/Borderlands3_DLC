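; Mission actor for "Big Expectation" (EP06), driving its chain of objectives from killing the fairy to fleeing through the fountain.
; After a short delay or the player MissionSystemComponent's starter event, it checks whether the mission is active and sets the first objective.
; Each MissionObserverListenerEvent advances the objective enum, mirrors it into ObjectiveInteger, then refreshes the HUD text and waypoint.
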(event Custom|MissionStarterActivator_Event_0
  (bind _missionisactive (CallFunction|CheckifMissionIsActive "NewEnumerator5"))
  (if _missionisactive
    (Variables|Default|SetMissionObjectives "NewEnumerator14")
    (Utilities|EnumBigeExpectationGC)
    (CallFunction|UpdateHUDTitleandObjective "Big Expectation" "Kill the fairy")
    (Default|CallMissionWaypointUpdate)))

(event EventBeginPlay
  (Utilities|FlowControl|Delay 1.0)
  (bind _asfirst_person_character (Utilities|Casting|CastToFirstPersonCharacter (Game|Player|GetPlayerPawn 0)))
  (Variables|Default|SetPlayerRef _asfirst_person_character)
  (Variables|Default|SetMOHUDRef (Variables|/Game/_FirstPersonBaseFiles/ProjectBasics/FirstPersonCharacter.FirstPersonCharacter_C|GetMissionObjectives_HUD _asfirst_person_character))
  (EventDispatchers|AssignMissionStarterActivator (Variables|/Game/_FirstPersonBaseFiles/ProjectBasics/FirstPersonCharacter.FirstPersonCharacter_C|GetMissionSystem_Component (Variables|Default|GetPlayerRef)) (delegate Custom|MissionStarterActivator_Event_0))
  (bind _missionisactive (CallFunction|CheckifMissionIsActive "NewEnumerator5"))
  (if _missionisactive
    (Variables|Default|SetMissionObjectives "NewEnumerator14")
    (Utilities|EnumBigeExpectationGC)
    (CallFunction|UpdateHUDTitleandObjective "Big Expectation" "Kill the fairy")
    (Default|CallMissionWaypointUpdate)))

(event EventMissionObserverListenerEvent
  (switch Utilities|FlowControl|Switch|SwitchonEnumGiantCastle (Variables|Default|GetMissionObjectives)
    (:NewEnumerator14
      (Variables|Default|SetMissionObjectives "NewEnumerator13")
      (Utilities|EnumBigeExpectationGC)
      (CallFunction|UpdateHUDTitleandObjective "Big Expectation" "Plant the bean")
      (Default|CallMissionWaypointUpdate))
    (:NewEnumerator13
      (Variables|Default|SetMissionObjectives "NewEnumerator12")
      (Utilities|EnumBigeExpectationGC)
      (CallFunction|UpdateHUDTitleandObjective "Big Expectation" "Defend the Bean")
      (Default|CallMissionWaypointUpdate))
    (:NewEnumerator12
      (Variables|Default|SetMissionObjectives "NewEnumerator11")
      (Utilities|EnumBigeExpectationGC)
      (CallFunction|UpdateHUDTitleandObjective "Big Expectation" "Reach the clouds")
      (Default|CallMissionWaypointUpdate))
    (:NewEnumerator11
      (Variables|Default|SetMissionObjectives "NewEnumerator0")
      (Utilities|EnumBigeExpectationGC)
      (CallFunction|UpdateHUDTitleandObjective "Big Expectation" "Reach the castle")
      (Default|CallMissionWaypointUpdate))
    (:NewEnumerator0
      (Variables|Default|SetMissionObjectives "NewEnumerator1")
      (Utilities|EnumBigeExpectationGC)
      (CallFunction|UpdateHUDTitleandObjective "Big Expectation" "Go talk to the hooded stranger")
      (Default|CallMissionWaypointUpdate))
    (:NewEnumerator1
      (Variables|Default|SetMissionObjectives "NewEnumerator2")
      (Utilities|EnumBigeExpectationGC)
      (CallFunction|UpdateHUDTitleandObjective "Big Expectation" "Defend Jack")
      (Default|CallMissionWaypointUpdate))
    (:NewEnumerator2
      (Variables|Default|SetMissionObjectives "NewEnumerator3")
      (Utilities|EnumBigeExpectationGC)
      (CallFunction|UpdateHUDTitleandObjective "Big Expectation" "Follow jack")
      (Default|CallMissionWaypointUpdate))
    (:NewEnumerator3
      (Variables|Default|SetMissionObjectives "NewEnumerator4")
      (Utilities|EnumBigeExpectationGC)
      (CallFunction|UpdateHUDTitleandObjective "Big Expectation" "Go fetch the helmet")
      (Default|CallMissionWaypointUpdate))
    (:NewEnumerator4
      (Variables|Default|SetMissionObjectives "NewEnumerator5")
      (Utilities|EnumBigeExpectationGC)
      (CallFunction|UpdateHUDTitleandObjective "Big Expectation" "Kill the thief")
      (Default|CallMissionWaypointUpdate))
    (:NewEnumerator5
      (Variables|Default|SetMissionObjectives "NewEnumerator6")
      (Utilities|EnumBigeExpectationGC)
      (CallFunction|UpdateHUDTitleandObjective "Big Expectation" "Bring the helmet to Jack")
      (Default|CallMissionWaypointUpdate))
    (:NewEnumerator6
      (Variables|Default|SetMissionObjectives "NewEnumerator7")
      (Utilities|EnumBigeExpectationGC)
      (CallFunction|UpdateHUDTitleandObjective "Big Expectation" "Kill Jack and his new minion")
      (Default|CallMissionWaypointUpdate))
    (:NewEnumerator7
      (Variables|Default|SetMissionObjectives "NewEnumerator8")
      (Utilities|EnumBigeExpectationGC)
      (CallFunction|UpdateHUDTitleandObjective "Big Expectation" "Flee through the fountain")
      (Default|CallMissionWaypointUpdate))
    (:NewEnumerator8
      (Variables|Default|SetMissionObjectives "NewEnumerator10")
      (Utilities|EnumBigeExpectationGC)
      (CallFunction|UpdateHUDTitleandObjective "Big Expectation" "Mission completed")
      (Default|CallMissionWaypointUpdate))))

(fn ConstructionScript
  (|CallParentFunction))