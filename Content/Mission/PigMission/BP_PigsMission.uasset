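; Mission actor for the "Three Little Psycho Pigs" quest, stepping through twenty linear objectives from talking to Tannis to completion.
; On BeginPlay it binds to the player's MissionSystemComponent starter event and, if the mission is active, sets the first objective.
; Each MissionObserverListenerEvent call advances the MissionObjectif enum by one step.
; Every step mirrors the enum into ObjectiveInteger, then updates the HUD text and mission waypoint.
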(event Custom|MissionStarterActivator_Event_0
  (bind _missionisactive (CallFunction|CheckifMissionIsActive "NewEnumerator3"))
  (if _missionisactive
    (Variables|Default|SetMissionObjectif "NewEnumerator1")
    (Utilities|EnumIntegerUpdate)
    (CallFunction|UpdateHUDTitleandObjective (Variables|Default|GetThree%20little%20psycho%20pigs) (Variables|Default|GetTalk%20to%20Tannis))
    (Default|CallMissionWaypointUpdate)))

(event EventBeginPlay
  (Utilities|FlowControl|Delay 1.0)
  (bind _asfirst_person_character (Utilities|Casting|CastToFirstPersonCharacter (Game|Player|GetPlayerPawn 0)))
  (Variables|Default|SetPlayer%20Ref _asfirst_person_character)
  (Variables|Default|SetMODHUDRef (Variables|/Game/_FirstPersonBaseFiles/ProjectBasics/FirstPersonCharacter.FirstPersonCharacter_C|GetMissionObjectives_HUD _asfirst_person_character))
  (EventDispatchers|AssignMissionStarterActivator (Variables|/Game/_FirstPersonBaseFiles/ProjectBasics/FirstPersonCharacter.FirstPersonCharacter_C|GetMissionSystem_Component (Variables|Default|GetPlayer%20Ref)) (delegate Custom|MissionStarterActivator_Event_0))
  (bind _missionisactive (CallFunction|CheckifMissionIsActive "NewEnumerator3"))
  (if _missionisactive
    (Variables|Default|SetMissionObjectif "NewEnumerator1")
    (Utilities|EnumIntegerUpdate)
    (CallFunction|UpdateHUDTitleandObjective (Variables|Default|GetThree%20little%20psycho%20pigs) (Variables|Default|GetTalk%20to%20Tannis))
    (Default|CallMissionWaypointUpdate)))

(event EventMissionObserverListenerEvent
  (switch Utilities|FlowControl|Switch|SwitchonENUM_Pigs (Variables|Default|GetMissionObjectif)
    (:NewEnumerator1
      (Variables|Default|SetMissionObjectif "NewEnumerator2")
      (Utilities|EnumIntegerUpdate)
      (CallFunction|UpdateHUDTitleandObjective (Variables|Default|GetThree%20little%20psycho%20pigs) (Variables|Default|GetTravel%20to%20Pigs%20Farm))
      (Default|CallMissionWaypointUpdate))
    (:NewEnumerator2
      (Variables|Default|SetMissionObjectif "NewEnumerator4")
      (Utilities|EnumIntegerUpdate)
      (CallFunction|UpdateHUDTitleandObjective (Variables|Default|GetThree%20little%20psycho%20pigs) (Variables|Default|GetConvince%20Farmers))
      (Default|CallMissionWaypointUpdate))
    (:NewEnumerator4
      (Variables|Default|SetMissionObjectif "NewEnumerator5")
      (Utilities|EnumIntegerUpdate)
      (CallFunction|UpdateHUDTitleandObjective (Variables|Default|GetThree%20little%20psycho%20pigs) (Variables|Default|GetKill%20the%20Creatures%20in%20the%20Turnips%20field))
      (Default|CallMissionWaypointUpdate))
    (:NewEnumerator5
      (Variables|Default|SetMissionObjectif "NewEnumerator6")
      (Utilities|EnumIntegerUpdate)
      (CallFunction|UpdateHUDTitleandObjective (Variables|Default|GetThree%20little%20psycho%20pigs) (Variables|Default|GetDefeat%20Oswald))
      (Default|CallMissionWaypointUpdate))
    (:NewEnumerator6
      (Variables|Default|SetMissionObjectif "NewEnumerator7")
      (Utilities|EnumIntegerUpdate)
      (CallFunction|UpdateHUDTitleandObjective (Variables|Default|GetThree%20little%20psycho%20pigs) (Variables|Default|GetObtain%20the%20Eridium%20scythe))
      (Default|CallMissionWaypointUpdate))
    (:NewEnumerator7
      (Variables|Default|SetMissionObjectif "NewEnumerator8")
      (Utilities|EnumIntegerUpdate)
      (CallFunction|UpdateHUDTitleandObjective (Variables|Default|GetThree%20little%20psycho%20pigs) (Variables|Default|GetDestroy%20the%20hay%20wall))
      (Default|CallMissionWaypointUpdate))
    (:NewEnumerator8
      (Variables|Default|SetMissionObjectif "NewEnumerator9")
      (Utilities|EnumIntegerUpdate)
      (CallFunction|UpdateHUDTitleandObjective (Variables|Default|GetThree%20little%20psycho%20pigs) (Variables|Default|GetConvince%20the%20workers))
      (Default|CallMissionWaypointUpdate))
    (:NewEnumerator9
      (Variables|Default|SetMissionObjectif "NewEnumerator10")
      (Utilities|EnumIntegerUpdate)
      (CallFunction|UpdateHUDTitleandObjective (Variables|Default|GetThree%20little%20psycho%20pigs) (Variables|Default|GetDefend%20the%20wood%20village))
      (Default|CallMissionWaypointUpdate))
    (:NewEnumerator10
      (Variables|Default|SetMissionObjectif "NewEnumerator11")
      (Utilities|EnumIntegerUpdate)
      (CallFunction|UpdateHUDTitleandObjective (Variables|Default|GetThree%20little%20psycho%20pigs) (Variables|Default|GetDefeat%20Larry))
      (Default|CallMissionWaypointUpdate))
    (:NewEnumerator11
      (Variables|Default|SetMissionObjectif "NewEnumerator12")
      (Utilities|EnumIntegerUpdate)
      (CallFunction|UpdateHUDTitleandObjective (Variables|Default|GetThree%20little%20psycho%20pigs) (Variables|Default|GetObtain%20the%20Eridium%20axe))
      (Default|CallMissionWaypointUpdate))
    (:NewEnumerator12
      (Variables|Default|SetMissionObjectif "NewEnumerator13")
      (Utilities|EnumIntegerUpdate)
      (CallFunction|UpdateHUDTitleandObjective (Variables|Default|GetThree%20little%20psycho%20pigs) (Variables|Default|GetDestroy%20the%20wood%20wall))
      (Default|CallMissionWaypointUpdate))
    (:NewEnumerator13
      (Variables|Default|SetMissionObjectif "NewEnumerator14")
      (Utilities|EnumIntegerUpdate)
      (CallFunction|UpdateHUDTitleandObjective (Variables|Default|GetThree%20little%20psycho%20pigs) (Variables|Default|GetConvince%20the%20peasants))
      (Default|CallMissionWaypointUpdate))
    (:NewEnumerator14
      (Variables|Default|SetMissionObjectif "NewEnumerator15")
      (Utilities|EnumIntegerUpdate)
      (CallFunction|UpdateHUDTitleandObjective (Variables|Default|GetThree%20little%20psycho%20pigs) (Variables|Default|GetDestroy%20the%20Wolfgang's%20barracks))
      (Default|CallMissionWaypointUpdate))
    (:NewEnumerator15
      (Variables|Default|SetMissionObjectif "NewEnumerator16")
      (Utilities|EnumIntegerUpdate)
      (CallFunction|UpdateHUDTitleandObjective (Variables|Default|GetThree%20little%20psycho%20pigs) (Variables|Default|GetDefeat%20Bubba))
      (Default|CallMissionWaypointUpdate))
    (:NewEnumerator16
      (Variables|Default|SetMissionObjectif "NewEnumerator17")
      (Utilities|EnumIntegerUpdate)
      (CallFunction|UpdateHUDTitleandObjective (Variables|Default|GetThree%20little%20psycho%20pigs) (Variables|Default|GetObtain%20the%20Eridium%20explosives))
      (Default|CallMissionWaypointUpdate))
    (:NewEnumerator17
      (Variables|Default|SetMissionObjectif "NewEnumerator18")
      (Utilities|EnumIntegerUpdate)
      (CallFunction|UpdateHUDTitleandObjective (Variables|Default|GetThree%20little%20psycho%20pigs) (Variables|Default|GetDestroy%20the%20reinforced%20wall))
      (Default|CallMissionWaypointUpdate))
    (:NewEnumerator18
      (Variables|Default|SetMissionObjectif "NewEnumerator19")
      (Utilities|EnumIntegerUpdate)
      (CallFunction|UpdateHUDTitleandObjective (Variables|Default|GetThree%20little%20psycho%20pigs) (Variables|Default|GetGo%20inside%20the%20palace))
      (Default|CallMissionWaypointUpdate))
    (:NewEnumerator19
      (Variables|Default|SetMissionObjectif "NewEnumerator20")
      (Utilities|EnumIntegerUpdate)
      (CallFunction|UpdateHUDTitleandObjective (Variables|Default|GetThree%20little%20psycho%20pigs) (Variables|Default|GetDefeat%20PiggyBot))
      (Default|CallMissionWaypointUpdate))
    (:NewEnumerator20
      (Variables|Default|SetMissionObjectif "NewEnumerator21")
      (Utilities|EnumIntegerUpdate)
      (CallFunction|UpdateHUDTitleandObjective (Variables|Default|GetThree%20little%20psycho%20pigs) (Variables|Default|GetTravel%20to%20the%20Park))
      (Default|CallMissionWaypointUpdate))
    (:NewEnumerator21
      (Variables|Default|SetMissionObjectif "NewEnumerator22")
      (Utilities|EnumIntegerUpdate)
      (CallFunction|UpdateHUDTitleandObjective (Variables|Default|GetThree%20little%20psycho%20pigs) (Variables|Default|GetMission%20Complete))
      (Default|CallMissionWaypointUpdate))))

(fn ConstructionScript
  (|CallParentFunction))