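; Mission actor for the Lagoon mission "The Little Fish Woman", stepping the player through a linear objective chain from finding the Fairy Gunmother to mission completion.
; On BeginPlay it registers an activation callback with the player's MissionSystemComponent and starts the first objective if the mission is active.
; Each observer event advances the objective enum, maps it to an integer via the EnumIntegerUpdate macro, then refreshes HUD text and waypoint.
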(event Custom|CheckIfMissionIsActivated
  (bind _missionisactive (CallFunction|CheckifMissionIsActive "NewEnumerator0"))
  (if _missionisactive
    (Variables|Default|SetMissionObjectives "NewEnumerator1")
    (Utilities|EnumIntegerUpdate
      (:Output
        (CallFunction|UpdateHUDTitleandObjective (Variables|Default|GetThe%20Little%20Fish%20Woman) (Variables|Default|GetFind%20Fairy%20Gunmother))
        (Default|CallMissionWaypointUpdate)))))

(event EventBeginPlay
  (Utilities|FlowControl|Delay 1.0)
  (bind _asfirst_person_character (Utilities|Casting|CastToFirstPersonCharacter (Game|Player|GetPlayerPawn 0)))
  (Variables|Default|SetPlayerRef _asfirst_person_character)
  (Variables|Default|SetMOHUDRef (Variables|/Game/_FirstPersonBaseFiles/ProjectBasics/FirstPersonCharacter.FirstPersonCharacter_C|GetMissionObjectives_HUD _asfirst_person_character))
  (EventDispatchers|AssignMissionStarterActivator (Variables|/Game/_FirstPersonBaseFiles/ProjectBasics/FirstPersonCharacter.FirstPersonCharacter_C|GetMissionSystem_Component (Variables|Default|GetPlayerRef)) (delegate Custom|CheckIfMissionIsActivated))
  (bind _missionisactive (CallFunction|CheckifMissionIsActive "NewEnumerator0"))
  (if _missionisactive
    (Variables|Default|SetMissionObjectives "NewEnumerator1")
    (Utilities|EnumIntegerUpdate
      (:Output
        (CallFunction|UpdateHUDTitleandObjective (Variables|Default|GetThe%20Little%20Fish%20Woman) (Variables|Default|GetFind%20Fairy%20Gunmother))
        (Default|CallMissionWaypointUpdate)))))

(event Collision|EventActorBeginOverlap
  (params (OtherActor :type Actor%20Object%20Reference))
  (|CallParentFunction OtherActor) ; This node is disabled and will not be called.\nDrag off pins to build functionality.
)

(event EventTick
  (params (DeltaSeconds :type Float%20%28single-precision%29))
  (|CallParentFunction DeltaSeconds) ; This node is disabled and will not be called.\nDrag off pins to build functionality.
)

(event EventMissionObserverListenerEvent
  (switch Utilities|FlowControl|Switch|SwitchonEnum_Lagoon_Objectives (Variables|Default|GetMissionObjectives)
    (:NewEnumerator1
      (Variables|Default|SetMissionObjectives "NewEnumerator2")
      (Utilities|EnumIntegerUpdate
        (:Output
          (CallFunction|UpdateHUDTitleandObjective (Variables|Default|GetThe%20Little%20Fish%20Woman) (Variables|Default|GetGo%20to%20the%20Blue%20Lagoon))
          (Default|CallMissionWaypointUpdate))))
    (:NewEnumerator2
      (Variables|Default|SetMissionObjectives "NewEnumerator3")
      (Utilities|EnumIntegerUpdate
        (:Output
          (CallFunction|UpdateHUDTitleandObjective (Variables|Default|GetThe%20Little%20Fish%20Woman) (Variables|Default|GetInvestigate%20Mysterious%20Disappearances))
          (Default|CallMissionWaypointUpdate))))
    (:NewEnumerator3
      (Variables|Default|SetMissionObjectives "NewEnumerator4")
      (Utilities|EnumIntegerUpdate
        (:Output
          (CallFunction|UpdateHUDTitleandObjective (Variables|Default|GetThe%20Little%20Fish%20Woman) (Variables|Default|GetQuestion%20The%20Little%20Fish%20Woman))
          (Default|CallMissionWaypointUpdate))))
    (:NewEnumerator4
      (Variables|Default|SetMissionObjectives "NewEnumerator5")
      (Utilities|EnumIntegerUpdate
        (:Output
          (CallFunction|UpdateHUDTitleandObjective (Variables|Default|GetThe%20Little%20Fish%20Woman) (Variables|Default|GetCross%20The%20Coral%20Reef))
          (Default|CallMissionWaypointUpdate))))
    (:NewEnumerator5
      (Variables|Default|SetMissionObjectives "NewEnumerator6")
      (Utilities|EnumIntegerUpdate
        (:Output
          (CallFunction|UpdateHUDTitleandObjective (Variables|Default|GetThe%20Little%20Fish%20Woman) (Variables|Default|GetSurvive%20The%20Arena))
          (Default|CallMissionWaypointUpdate))))
    (:NewEnumerator6
      (Variables|Default|SetMissionObjectives "NewEnumerator7")
      (Utilities|EnumIntegerUpdate
        (:Output
          (CallFunction|UpdateHUDTitleandObjective (Variables|Default|GetThe%20Little%20Fish%20Woman) (Variables|Default|GetFree%20the%20Prisonners))
          (Default|CallMissionWaypointUpdate))))
    (:NewEnumerator7
      (Variables|Default|SetMissionObjectives "NewEnumerator8")
      (Utilities|EnumIntegerUpdate
        (:Output
          (CallFunction|UpdateHUDTitleandObjective (Variables|Default|GetThe%20Little%20Fish%20Woman) (Variables|Default|GetFollow%20The%20Trail%20of%20The%20Little%20Fish%20Woman))
          (Default|CallMissionWaypointUpdate))))
    (:NewEnumerator8
      (Variables|Default|SetMissionObjectives "NewEnumerator9")
      (Utilities|EnumIntegerUpdate
        (:Output
          (CallFunction|UpdateHUDTitleandObjective (Variables|Default|GetThe%20Little%20Fish%20Woman) (Variables|Default|GetFight%20The%20Little%20Fish%20Woman))
          (Default|CallMissionWaypointUpdate))))
    (:NewEnumerator9
      (Variables|Default|SetMissionObjectives "NewEnumerator10")
      (Utilities|EnumIntegerUpdate
        (:Output
          (CallFunction|UpdateHUDTitleandObjective (Variables|Default|GetThe%20Little%20Fish%20Woman) (Variables|Default|GetReturn%20To%20The%20Castle%20of%20The%20Fairy%20Gunmother))
          (Default|CallMissionWaypointUpdate))))
    (:NewEnumerator10
      (Variables|Default|SetMissionObjectives "NewEnumerator11")
      (Utilities|EnumIntegerUpdate
        (:Output
          (CallFunction|UpdateHUDTitleandObjective (Variables|Default|GetThe%20Little%20Fish%20Woman) (Variables|Default|GetMeet%20The%20Fairy%20Gunmother))
          (Default|CallMissionWaypointUpdate))))
    (:NewEnumerator11
      (Variables|Default|SetMissionObjectives "NewEnumerator12")
      (Utilities|EnumIntegerUpdate
        (:Output
          (CallFunction|UpdateHUDTitleandObjective (Variables|Default|GetThe%20Little%20Fish%20Woman) (Variables|Default|GetMission%20Complete))
          (Default|CallMissionWaypointUpdate))))))

(fn ConstructionScript
  (|CallParentFunction))