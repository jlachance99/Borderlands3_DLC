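; BP_Mission is a mission actor that provides shared helpers for querying mission state and updating the objectives HUD.
; Its construction script writes debug text to a TextRender component.
; Both helpers cast player pawn 0 to FirstPersonCharacter, one comparing its MissionSystemComponent's active mission, the other setting HUD title and first objective.
; Event handlers, including the mission observer listener, are empty, and the waypoint and objective dispatcher calls are unconnected.
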(event Custom|MissionObserverListener_Event)

(event EventBeginPlay)

(event Collision|EventActorBeginOverlap
  (params (OtherActor :type Actor%20Object%20Reference)))

(event EventTick
  (params (DeltaSeconds :type Float%20%28single-precision%29)))

(fn ConstructionScript
  (Rendering|Components|TextRender|SetText (Variables|Default|GetTextRender) (Variables|Debug|GetDebugRendererText)))

(fn CheckifMissionIsActive
  (params (MissionToCheck :type Enum_MissionList%20Enum :default "NewEnumerator0"))
  (bind _asfirst_person_character (Utilities|Casting|CastToFirstPersonCharacter (Game|Player|GetPlayerPawn 0)))
  (if (Utilities|Enum|Equal(Enum) (Variables|/Game/Mission/Components/MissionSystem_Component.MissionSystem_Component_C|GetActivatedMission (Variables|/Game/_FirstPersonBaseFiles/ProjectBasics/FirstPersonCharacter.FirstPersonCharacter_C|GetMissionSystem_Component _asfirst_person_character)) MissionToCheck)
    (return true)
    (else
      (return false))))

(fn UpdateHUDTitleandObjective
  (params (MissionTitle :type Text) (ObjectiveText :type Text))
  (bind _asfirst_person_character (Utilities|Casting|CastToFirstPersonCharacter (Game|Player|GetPlayerPawn 0)))
  (Default|MOHUDMissionTitle (Variables|/Game/_FirstPersonBaseFiles/ProjectBasics/FirstPersonCharacter.FirstPersonCharacter_C|GetMissionObjectives_HUD _asfirst_person_character) MissionTitle)
  (Default|MOHUDMissionObjective1 (Variables|/Game/_FirstPersonBaseFiles/ProjectBasics/FirstPersonCharacter.FirstPersonCharacter_C|GetMissionObjectives_HUD _asfirst_person_character) ObjectiveText))