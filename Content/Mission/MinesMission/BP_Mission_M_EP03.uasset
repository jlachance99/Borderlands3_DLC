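; Mission controller for the "Once Upon a mine" mines mission, stepping the player through 38 objectives to completion.
; After a BeginPlay delay it registers with the player's MissionSystemComponent and sets the first objective if the mission is active.
; Each MissionObserverListenerEvent advances the objective enum, mirrors it to an integer, and updates HUD text and waypoint.
; From objective 35 onward, HUD text variables are out of step with the enum.
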(event Custom|CheckIfMissionIsActivated
  (bind _missionisactive (CallFunction|CheckifMissionIsActive "NewEnumerator2"))
  (if _missionisactive
    (Variables|Default|SetMissionObjectives "NewEnumerator1")
    (Utilities|EnumIntegerUpdate
      (:Output
        (CallFunction|UpdateHUDTitleandObjective "Once Upon a mine" (Variables|Default|GetObjective1))
        (Default|CallMissionWaypointUpdate)))))

(event EventBeginPlay
  (Utilities|FlowControl|Delay 1.0)
  (bind _asfirst_person_character (Utilities|Casting|CastToFirstPersonCharacter (Game|Player|GetPlayerPawn 0)))
  (Variables|Default|SetPlayerRef _asfirst_person_character)
  (Variables|Default|SetMOHUDRef (Variables|/Game/_FirstPersonBaseFiles/ProjectBasics/FirstPersonCharacter.FirstPersonCharacter_C|GetMissionObjectives_HUD _asfirst_person_character))
  (EventDispatchers|AssignMissionStarterActivator (Variables|/Game/_FirstPersonBaseFiles/ProjectBasics/FirstPersonCharacter.FirstPersonCharacter_C|GetMissionSystem_Component (Variables|Default|GetPlayerRef)) (delegate Custom|CheckIfMissionIsActivated))
  (bind _missionisactive (CallFunction|CheckifMissionIsActive "NewEnumerator2"))
  (if _missionisactive
    (Variables|Default|SetMissionObjectives "NewEnumerator1")
    (Utilities|EnumIntegerUpdate
      (:Output
        (CallFunction|UpdateHUDTitleandObjective "Once Upon a mine" (Variables|Default|GetObjective1))
        (Default|CallMissionWaypointUpdate)))))

(event Collision|EventActorBeginOverlap
  (params (OtherActor :type Actor%20Object%20Reference))
  (|CallParentFunction OtherActor) ; This node is disabled and will not be called.\nDrag off pins to build functionality.
)

(event EventMissionObserverListenerEvent
  (switch Utilities|FlowControl|Switch|SwitchonEnum_Mines_Objectives (Variables|Default|GetMissionObjectives)
    (:NewEnumerator1
      (Variables|Default|SetMissionObjectives "NewEnumerator2")
      (Utilities|EnumIntegerUpdate
        (:Output
          (CallFunction|UpdateHUDTitleandObjective "Once Upon a mine" (Variables|Default|GetObjective2))
          (Default|CallMissionWaypointUpdate))))
    (:NewEnumerator2
      (Variables|Default|SetMissionObjectives "NewEnumerator4")
      (Utilities|EnumIntegerUpdate
        (:Output
          (CallFunction|UpdateHUDTitleandObjective "Once Upon a mine" (Variables|Default|GetObjective3))
          (Default|CallMissionWaypointUpdate))))
    (:NewEnumerator4
      (Variables|Default|SetMissionObjectives "NewEnumerator5")
      (Utilities|EnumIntegerUpdate
        (:Output
          (CallFunction|UpdateHUDTitleandObjective "Once Upon a mine" (Variables|Default|GetObjective4))
          (Default|CallMissionWaypointUpdate))))
    (:NewEnumerator5
      (Variables|Default|SetMissionObjectives "NewEnumerator6")
      (Utilities|EnumIntegerUpdate
        (:Output
          (CallFunction|UpdateHUDTitleandObjective "Once Upon a mine" (Variables|Default|GetObjective5))
          (Default|CallMissionWaypointUpdate))))
    (:NewEnumerator6
      (Variables|Default|SetMissionObjectives "NewEnumerator7")
      (Utilities|EnumIntegerUpdate
        (:Output
          (CallFunction|UpdateHUDTitleandObjective "Once Upon a mine" (Variables|Default|GetObjective6))
          (Default|CallMissionWaypointUpdate))))
    (:NewEnumerator7
      (Variables|Default|SetMissionObjectives "NewEnumerator8")
      (Utilities|EnumIntegerUpdate
        (:Output
          (CallFunction|UpdateHUDTitleandObjective "Once Upon a mine" (Variables|Default|GetObjective7))
          (Default|CallMissionWaypointUpdate))))
    (:NewEnumerator8
      (Variables|Default|SetMissionObjectives "NewEnumerator9")
      (Utilities|EnumIntegerUpdate
        (:Output
          (CallFunction|UpdateHUDTitleandObjective "Once Upon a mine" (Variables|Default|GetObjective8))
          (Default|CallMissionWaypointUpdate))))
    (:NewEnumerator9
      (Variables|Default|SetMissionObjectives "NewEnumerator10")
      (Utilities|EnumIntegerUpdate
        (:Output
          (CallFunction|UpdateHUDTitleandObjective "Once Upon a mine" (Variables|Default|GetObjective9))
          (Default|CallMissionWaypointUpdate))))
    (:NewEnumerator10
      (Variables|Default|SetMissionObjectives "NewEnumerator11")
      (Utilities|EnumIntegerUpdate
        (:Output
          (CallFunction|UpdateHUDTitleandObjective "Once Upon a mine" (Variables|Default|GetObjective10))
          (Default|CallMissionWaypointUpdate))))
    (:NewEnumerator11
      (Variables|Default|SetMissionObjectives "NewEnumerator12")
      (Utilities|EnumIntegerUpdate
        (:Output
          (CallFunction|UpdateHUDTitleandObjective "Once Upon a mine" (Variables|Default|GetObjective11))
          (Default|CallMissionWaypointUpdate))))
    (:NewEnumerator12
      (Variables|Default|SetMissionObjectives "NewEnumerator13")
      (Utilities|EnumIntegerUpdate
        (:Output
          (CallFunction|UpdateHUDTitleandObjective "Once Upon a mine" (Variables|Default|GetObjective12))
          (Default|CallMissionWaypointUpdate))))
    (:NewEnumerator13
      (Variables|Default|SetMissionObjectives "NewEnumerator14")
      (Utilities|EnumIntegerUpdate
        (:Output
          (CallFunction|UpdateHUDTitleandObjective "Once Upon a mine" (Variables|Default|GetObjective13))
          (Default|CallMissionWaypointUpdate))))
    (:NewEnumerator14
      (Variables|Default|SetMissionObjectives "NewEnumerator15")
      (Utilities|EnumIntegerUpdate
        (:Output
          (CallFunction|UpdateHUDTitleandObjective "Once Upon a mine" (Variables|Default|GetObjective14))
          (Default|CallMissionWaypointUpdate))))
    (:NewEnumerator15
      (Variables|Default|SetMissionObjectives "NewEnumerator16")
      (Utilities|EnumIntegerUpdate
        (:Output
          (CallFunction|UpdateHUDTitleandObjective "Once Upon a mine" (Variables|Default|GetObjective15))
          (Default|CallMissionWaypointUpdate))))
    (:NewEnumerator16
      (Variables|Default|SetMissionObjectives "NewEnumerator17")
      (Utilities|EnumIntegerUpdate
        (:Output
          (CallFunction|UpdateHUDTitleandObjective "Once Upon a mine" (Variables|Default|GetObjective16))
          (Default|CallMissionWaypointUpdate))))
    (:NewEnumerator17
      (Variables|Default|SetMissionObjectives "NewEnumerator18")
      (Utilities|EnumIntegerUpdate
        (:Output
          (CallFunction|UpdateHUDTitleandObjective "Once Upon a mine" (Variables|Default|GetObjective17))
          (Default|CallMissionWaypointUpdate))))
    (:NewEnumerator18
      (Variables|Default|SetMissionObjectives "NewEnumerator19")
      (Utilities|EnumIntegerUpdate
        (:Output
          (CallFunction|UpdateHUDTitleandObjective "Once Upon a mine" (Variables|Default|GetObjective18))
          (Default|CallMissionWaypointUpdate))))
    (:NewEnumerator19
      (Variables|Default|SetMissionObjectives "NewEnumerator20")
      (Utilities|EnumIntegerUpdate
        (:Output
          (CallFunction|UpdateHUDTitleandObjective "Once Upon a mine" (Variables|Default|GetObjective19))
          (Default|CallMissionWaypointUpdate))))
    (:NewEnumerator20
      (Variables|Default|SetMissionObjectives "NewEnumerator21")
      (Utilities|EnumIntegerUpdate
        (:Output
          (CallFunction|UpdateHUDTitleandObjective "Once Upon a mine" (Variables|Default|GetObjective20))
          (Default|CallMissionWaypointUpdate))))
    (:NewEnumerator21
      (Variables|Default|SetMissionObjectives "NewEnumerator22")
      (Utilities|EnumIntegerUpdate
        (:Output
          (CallFunction|UpdateHUDTitleandObjective "Once Upon a mine" (Variables|Default|GetObjective21))
          (Default|CallMissionWaypointUpdate))))
    (:NewEnumerator22
      (Variables|Default|SetMissionObjectives "NewEnumerator23")
      (Utilities|EnumIntegerUpdate
        (:Output
          (CallFunction|UpdateHUDTitleandObjective "Once Upon a mine" (Variables|Default|GetObjective22))
          (Default|CallMissionWaypointUpdate))))
    (:NewEnumerator23
      (Variables|Default|SetMissionObjectives "NewEnumerator24")
      (Utilities|EnumIntegerUpdate
        (:Output
          (CallFunction|UpdateHUDTitleandObjective "Once Upon a mine" (Variables|Default|GetObjective23))
          (Default|CallMissionWaypointUpdate))))
    (:NewEnumerator24
      (Variables|Default|SetMissionObjectives "NewEnumerator25")
      (Utilities|EnumIntegerUpdate
        (:Output
          (CallFunction|UpdateHUDTitleandObjective "Once Upon a mine" (Variables|Default|GetObjective24))
          (Default|CallMissionWaypointUpdate))))
    (:NewEnumerator25
      (Variables|Default|SetMissionObjectives "NewEnumerator26")
      (Utilities|EnumIntegerUpdate
        (:Output
          (CallFunction|UpdateHUDTitleandObjective "Once Upon a mine" (Variables|Default|GetObjective25))
          (Default|CallMissionWaypointUpdate))))
    (:NewEnumerator26
      (Variables|Default|SetMissionObjectives "NewEnumerator27")
      (Utilities|EnumIntegerUpdate
        (:Output
          (CallFunction|UpdateHUDTitleandObjective "Once Upon a mine" (Variables|Default|GetObjective26))
          (Default|CallMissionWaypointUpdate))))
    (:NewEnumerator27
      (Variables|Default|SetMissionObjectives "NewEnumerator28")
      (Utilities|EnumIntegerUpdate
        (:Output
          (CallFunction|UpdateHUDTitleandObjective "Once Upon a mine" (Variables|Default|GetObjective27))
          (Default|CallMissionWaypointUpdate))))
    (:NewEnumerator28
      (Variables|Default|SetMissionObjectives "NewEnumerator29")
      (Utilities|EnumIntegerUpdate
        (:Output
          (CallFunction|UpdateHUDTitleandObjective "Once Upon a mine" (Variables|Default|GetObjective28))
          (Default|CallMissionWaypointUpdate))))
    (:NewEnumerator29
      (Variables|Default|SetMissionObjectives "NewEnumerator30")
      (Utilities|EnumIntegerUpdate
        (:Output
          (CallFunction|UpdateHUDTitleandObjective "Once Upon a mine" (Variables|Default|GetObjective29))
          (Default|CallMissionWaypointUpdate))))
    (:NewEnumerator30
      (Variables|Default|SetMissionObjectives "NewEnumerator31")
      (Utilities|EnumIntegerUpdate
        (:Output
          (CallFunction|UpdateHUDTitleandObjective "Once Upon a mine" (Variables|Default|GetObjective30))
          (Default|CallMissionWaypointUpdate))))
    (:NewEnumerator31
      (Variables|Default|SetMissionObjectives "NewEnumerator32")
      (Utilities|EnumIntegerUpdate
        (:Output
          (CallFunction|UpdateHUDTitleandObjective "Once Upon a mine" (Variables|Default|GetObjective31))
          (Default|CallMissionWaypointUpdate))))
    (:NewEnumerator32
      (Variables|Default|SetMissionObjectives "NewEnumerator33")
      (Utilities|EnumIntegerUpdate
        (:Output
          (CallFunction|UpdateHUDTitleandObjective "Once Upon a mine" (Variables|Default|GetObjective32))
          (Default|CallMissionWaypointUpdate))))
    (:NewEnumerator33
      (Variables|Default|SetMissionObjectives "NewEnumerator34")
      (Utilities|EnumIntegerUpdate
        (:Output
          (CallFunction|UpdateHUDTitleandObjective "Once Upon a mine" (Variables|Default|GetObjective33))
          (Default|CallMissionWaypointUpdate))))
    (:NewEnumerator34
      (Variables|Default|SetMissionObjectives "NewEnumerator35")
      (Utilities|EnumIntegerUpdate
        (:Output
          (CallFunction|UpdateHUDTitleandObjective "Once Upon a mine" (Variables|Default|GetObjective34))
          (Default|CallMissionWaypointUpdate))))
    (:NewEnumerator35
      (Variables|Default|SetMissionObjectives "NewEnumerator40")
      (Utilities|EnumIntegerUpdate
        (:Output
          (CallFunction|UpdateHUDTitleandObjective "Once Upon a mine" (Variables|Default|GetObjective39))
          (Default|CallMissionWaypointUpdate))))
    (:NewEnumerator40
      (Variables|Default|SetMissionObjectives "NewEnumerator36")
      (Utilities|EnumIntegerUpdate
        (:Output
          (CallFunction|UpdateHUDTitleandObjective "Once Upon a mine" (Variables|Default|GetObjective35))
          (Default|CallMissionWaypointUpdate))))
    (:NewEnumerator36
      (Variables|Default|SetMissionObjectives "NewEnumerator37")
      (Utilities|EnumIntegerUpdate
        (:Output
          (CallFunction|UpdateHUDTitleandObjective "Once Upon a mine" (Variables|Default|GetObjective36))
          (Default|CallMissionWaypointUpdate))))
    (:NewEnumerator37
      (Variables|Default|SetMissionObjectives "NewEnumerator39")
      (Utilities|EnumIntegerUpdate
        (:Output
          (CallFunction|UpdateHUDTitleandObjective "Once Upon a mine" (Variables|Default|GetObjective37))
          (Default|CallMissionWaypointUpdate))))
    (:NewEnumerator39
      (Variables|Default|SetMissionObjectives "NewEnumerator3")
      (Utilities|EnumIntegerUpdate
        (:Output
          (CallFunction|UpdateHUDTitleandObjective "Once Upon a mine" (Variables|Default|GetObjective38))
          (Default|CallMissionWaypointUpdate))))))

(event EventTick
  (params (DeltaSeconds :type Float%20%28single-precision%29))
  (|CallParentFunction DeltaSeconds) ; This node is disabled and will not be called.\nDrag off pins to build functionality.
)

(fn ConstructionScript
  (|CallParentFunction))