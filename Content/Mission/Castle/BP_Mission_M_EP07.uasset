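; Mission controller for episode 7, "The Fairyest of Them All", stepping the player from talking to Tannis through the castle to defeating the Fairy Gun Mother.
; On BeginPlay, and whenever the player's MissionSystemComponent signals, it checks whether the mission is active and sets the first objective.
; MissionObserverListenerEvent advances the objective enum one step.
; Each change updates an integer mirror via a macro, then refreshes the HUD and waypoint.
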(event Custom|CheckIfMissionShouldBeActivated
  (bind _missionisactive (CallFunction|CheckifMissionIsActive "NewEnumerator6"))
  (if _missionisactive
    (Variables|Default|SetMissionObjectives "NewEnumerator2")
    (Utilities|EnumIntegerUpdate
      (:Output
        (CallFunction|UpdateHUDTitleandObjective (Variables|Default|GetThe%20Fairyest%20of%20them%20all) (Variables|Default|GetTalk%20to%20Tannis))
        (Default|CallMissionWaypointUpdate)))))

(event EventBeginPlay
  (Utilities|FlowControl|Delay 1.0)
  (bind _asfirst_person_character (Utilities|Casting|CastToFirstPersonCharacter (Game|Player|GetPlayerPawn 0)))
  (Variables|Default|SetPlayerRef _asfirst_person_character)
  (Variables|Default|SetMOHUDRef (Variables|/Game/_FirstPersonBaseFiles/ProjectBasics/FirstPersonCharacter.FirstPersonCharacter_C|GetMissionObjectives_HUD _asfirst_person_character))
  (EventDispatchers|BindEventtoMissionStarterActivator (Variables|/Game/_FirstPersonBaseFiles/ProjectBasics/FirstPersonCharacter.FirstPersonCharacter_C|GetMissionSystem_Component (Variables|Default|GetPlayerRef)) (delegate Custom|CheckIfMissionShouldBeActivated))
  (bind _missionisactive (CallFunction|CheckifMissionIsActive "NewEnumerator6"))
  (if _missionisactive
    (Variables|Default|SetMissionObjectives "NewEnumerator2")
    (Utilities|EnumIntegerUpdate
      (:Output
        (CallFunction|UpdateHUDTitleandObjective (Variables|Default|GetThe%20Fairyest%20of%20them%20all) (Variables|Default|GetTalk%20to%20Tannis))
        (Default|CallMissionWaypointUpdate)))))

(event EventMissionObserverListenerEvent
  (switch Utilities|FlowControl|Switch|SwitchonEnum_Castle_Objectives (Variables|Default|GetMissionObjectives)
    (:NewEnumerator2
      (Variables|Default|SetMissionObjectives "NewEnumerator12")
      (Utilities|EnumIntegerUpdate
        (:Output
          (CallFunction|UpdateHUDTitleandObjective (Variables|Default|GetThe%20Fairyest%20of%20them%20all) (Variables|Default|GetGo%20the%20the%20Fairy%20GunMother's%20Castle))
          (Default|CallMissionWaypointUpdate))))
    (:NewEnumerator12
      (Variables|Default|SetMissionObjectives "NewEnumerator3")
      (Utilities|EnumIntegerUpdate
        (:Output
          (CallFunction|UpdateHUDTitleandObjective (Variables|Default|GetThe%20Fairyest%20of%20them%20all) (Variables|Default|GetWalk%20the%20red%20carpet))
          (Default|CallMissionWaypointUpdate))))
    (:NewEnumerator3
      (Variables|Default|SetMissionObjectives "NewEnumerator4")
      (Utilities|EnumIntegerUpdate
        (:Output
          (CallFunction|UpdateHUDTitleandObjective (Variables|Default|GetThe%20Fairyest%20of%20them%20all) (Variables|Default|GetSurvive%20the%20paparazzis))
          (Default|CallMissionWaypointUpdate))))
    (:NewEnumerator4
      (Variables|Default|SetMissionObjectives "NewEnumerator5")
      (Utilities|EnumIntegerUpdate
        (:Output
          (CallFunction|UpdateHUDTitleandObjective (Variables|Default|GetThe%20Fairyest%20of%20them%20all) (Variables|Default|GetInfiltrate%20the%20ballroom))
          (Default|CallMissionWaypointUpdate))))
    (:NewEnumerator5
      (Variables|Default|SetMissionObjectives "NewEnumerator6")
      (Utilities|EnumIntegerUpdate
        (:Output
          (CallFunction|UpdateHUDTitleandObjective (Variables|Default|GetThe%20Fairyest%20of%20them%20all) (Variables|Default|GetGo%20to%20the%20second%20floor))
          (Default|CallMissionWaypointUpdate))))
    (:NewEnumerator6
      (Variables|Default|SetMissionObjectives "NewEnumerator7")
      (Utilities|EnumIntegerUpdate
        (:Output
          (CallFunction|UpdateHUDTitleandObjective (Variables|Default|GetThe%20Fairyest%20of%20them%20all) (Variables|Default|GetPass%20the%20chandeliers))
          (Default|CallMissionWaypointUpdate))))
    (:NewEnumerator7
      (Variables|Default|SetMissionObjectives "NewEnumerator8")
      (Utilities|EnumIntegerUpdate
        (:Output
          (CallFunction|UpdateHUDTitleandObjective (Variables|Default|GetThe%20Fairyest%20of%20them%20all) (Variables|Default|GetSurvive%20the%20art%20gallery))
          (Default|CallMissionWaypointUpdate))))
    (:NewEnumerator8
      (Variables|Default|SetMissionObjectives "NewEnumerator9")
      (Utilities|EnumIntegerUpdate
        (:Output
          (CallFunction|UpdateHUDTitleandObjective (Variables|Default|GetThe%20Fairyest%20of%20them%20all) (Variables|Default|GetKill%20the%20warehouse%20keeper))
          (Default|CallMissionWaypointUpdate))))
    (:NewEnumerator9
      (Variables|Default|SetMissionObjectives "NewEnumerator10")
      (Utilities|EnumIntegerUpdate
        (:Output
          (CallFunction|UpdateHUDTitleandObjective (Variables|Default|GetThe%20Fairyest%20of%20them%20all) (Variables|Default|GetFind%20the%20exit))
          (Default|CallMissionWaypointUpdate))))
    (:NewEnumerator10
      (Variables|Default|SetMissionObjectives "NewEnumerator1")
      (Utilities|EnumIntegerUpdate
        (:Output
          (CallFunction|UpdateHUDTitleandObjective (Variables|Default|GetThe%20Fairyest%20of%20them%20all) (Variables|Default|GetDefeat%20the%20Fairy%20GunMother))
          (Default|CallMissionWaypointUpdate))))
    (:NewEnumerator1
      (Variables|Default|SetMissionObjectives "NewEnumerator11")
      (Utilities|EnumIntegerUpdate
        (:Output
          (CallFunction|UpdateHUDTitleandObjective (Variables|Default|GetThe%20Fairyest%20of%20them%20all) (Variables|Default|GetMission%20End))
          (Default|CallMissionWaypointUpdate))))))

(fn ConstructionScript
  (|CallParentFunction))